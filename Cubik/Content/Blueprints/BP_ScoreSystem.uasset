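; BP_ScoreSystem keeps a time-based score for the duration of a run.
; When a run starts, it stores the player HUD and starts a looping timer that increments the score at a fixed short interval.
; Each tick of that timer pushes the new score to the HUD, and ending the run clears the timer to stop scoring.
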(event `OnRunStarted`
  (params (PlayerHUD :type "/Game/UI/WP_ScoreWidget Object Reference"))
  (set `self.PlayerHUDRef` PlayerHUD)
  (bind _returnvalue (`KismetSystemLibrary.K2_SetTimerDelegate` (delegate `CalculateScore`) 0.1 true))
  (set `self.ScoreTimerHandle` _returnvalue))

(event `CalculateScore`
  (bind _output_get (set `self.Score` (+ (`self.Score`) 1)))
  (`/Game/UI/WP_ScoreWidget.OnScoreChanged` (`self.PlayerHUDRef`) _output_get))

(event `OnRunEnded`
  (`KismetSystemLibrary.K2_ClearAndInvalidateTimerHandle` (`self.ScoreTimerHandle`)))

(fn `UserConstructionScript`)